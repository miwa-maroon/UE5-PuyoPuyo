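; BP_BloomGrassAlongSpline places grass and flower instanced meshes along a spline, with NumberWeight controlling how far along they fill.
; AddInstances spaces both meshes by the grass's X bounds plus Offset, orienting each toward the next point.
; It runs on construction and from Tick whenever NumberWeight differs from NumberWeightLast.
; The graphs never update NumberWeightLast or clear instances, so repeated runs stack duplicates.
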(event Custom|OnValueChanged
  (params (value :type Float%20%28double-precision%29))
  (Variables|Default|SetNumberWeight value)
  (CallFunction|AddInstances))

(event EventBeginPlay)

(event Collision|EventActorBeginOverlap
  (params (OtherActor :type Actor%20Object%20Reference)))

(event EventTick
  (params (DeltaSeconds :type Float%20%28single-precision%29))
  (bind _numberweight (Variables|Default|GetNumberWeight))
  (if (not (== _numberweight (Variables|Default|GetNumberWeightLast)))
    (CallFunction|OnValueChanged _numberweight)))

(fn ConstructionScript
  (Variables|Default|SetNumberWeight (Variables|Default|GetNumberWeight))
  (CallFunction|AddInstances))

(fn GetLocationatIndex
  (params (A :type Integer))
  (return (Spline|GetLocationatDistanceAlongSpline (Variables|Default|GetSpline) (* A (Variables|Default|GetSpacing)) "Local")))

(fn AddInstances
  (bind _grass (Variables|Default|GetGrass))
  (bind _returnvalue (StaticMesh|GetBoundingBox _grass))
  (bind (_min _max) (Utilities|Struct|BreakBox _returnvalue))
  (Components|StaticMesh|SetStaticMesh (Variables|Default|GetInstancedStaticMesh) (Variables|Default|GetGrass))
  (Components|StaticMesh|SetStaticMesh (Variables|Default|GetInstancedStaticMesh1) (Variables|Default|GetFlower))
  (bind _output_get (Variables|Default|SetSpacing (+ (.X (Math|Vector|BreakVector (- _max _min))) (Variables|Default|GetOffset))))
  (bind _output_get_2 (Variables|Default|SetNumberOfInstaces (Math|Float|Floor (/ (Spline|GetSplineLength (Variables|Default|GetSpline)) _output_get))))
  (for _index (range 0 (Math|Float|Round (* _output_get_2 (Variables|Default|GetNumberWeight))))
    (Components|InstancedStaticMesh|AddInstance (Variables|Default|GetInstancedStaticMesh) (Math|Transform|MakeTransform (CallFunction|GetLocationatIndex _index) (Math|Rotator|MakeRotfromX (- (CallFunction|GetLocationatIndex (+ _index 1)) (CallFunction|GetLocationatIndex _index)))) false)
    (Components|InstancedStaticMesh|AddInstance (Variables|Default|GetInstancedStaticMesh1) (Math|Transform|MakeTransform (CallFunction|GetLocationatIndex _index) (Math|Rotator|MakeRotfromX (- (CallFunction|GetLocationatIndex (+ _index 1)) (CallFunction|GetLocationatIndex _index)))) false)))