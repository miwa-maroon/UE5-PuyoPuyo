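; Puyo piece actor that shows links to neighboring pieces by deforming its MorphPuyoMesh with morph targets.
; BeginPlay sets both eye-blink morphs to full.
; Four directional events each set a connection morph to full, with vertical names inverted: MorphUp drives ConnectToBottom and MorphDown drives ConnectToTop.
; BacktoNormal clears all four connection morphs, leaving the blink morphs untouched.
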(event EventBeginPlay
  (bind _morphpuyomesh (Variables|Default|GetMorphPuyoMesh))
  (Components|SkeletalMesh|SetMorphTarget _morphpuyomesh "EyeBlinkLeft" 1.0 true)
  (Components|SkeletalMesh|SetMorphTarget _morphpuyomesh "EyeBlinkRight" 1.0 true))

(event Collision|EventActorBeginOverlap
  (params (OtherActor :type Actor%20Object%20Reference)))

(event EventTick
  (params (DeltaSeconds :type Float%20%28single-precision%29)))

(event EventMorphDown
  (Components|SkeletalMesh|SetMorphTarget (Variables|Default|GetMorphPuyoMesh) "ConnectToTop" 1.0 true))

(event EventMorphLeft
  (Components|SkeletalMesh|SetMorphTarget (Variables|Default|GetMorphPuyoMesh) "ConnectToLeft" 1.0 true))

(event EventMorphRight
  (Components|SkeletalMesh|SetMorphTarget (Variables|Default|GetMorphPuyoMesh) "ConnectToRight" 1.0 true))

(event EventMorphUp
  (Components|SkeletalMesh|SetMorphTarget (Variables|Default|GetMorphPuyoMesh) "ConnectToBottom" 1.0 true))

(event EventBacktoNormal
  (bind _morphpuyomesh (Variables|Default|GetMorphPuyoMesh))
  (Components|SkeletalMesh|SetMorphTarget _morphpuyomesh "ConnectToTop" 0.0 true)
  (Components|SkeletalMesh|SetMorphTarget _morphpuyomesh "ConnectToRight" 0.0 true)
  (Components|SkeletalMesh|SetMorphTarget _morphpuyomesh "ConnectToLeft" 0.0 true)
  (Components|SkeletalMesh|SetMorphTarget _morphpuyomesh "ConnectToBottom" 0.0 true))

(fn ConstructionScript)